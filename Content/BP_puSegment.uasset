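; BP_puSegment is a construction-time tool that repeats a template static mesh along a straight segment toward the end point of its spline.
; UpdateSegment derives direction and instance count from distance and Step, measuring from the InstancerComponent to that end point, ignoring curvature.
; The InstancerComponent pipeline generates serial transforms, applies optional target-facing rotation, randomizes location, rotation and scale, then realizes the instances.
; The construction script also snaps SMtarget to the spline end.
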(event EventBeginPlay)

(event Collision|EventActorBeginOverlap
  (params (OtherActor :type Actor%20Object%20Reference)))

(event EventTick
  (params (DeltaSeconds :type Float%20%28single-precision%29)))

(fn ConstructionScript
  (Components|StaticMesh|SetStaticMesh (Variables|Default|GetInstancerComponent) (Variables|Instancing|GetTemplateStaticMesh))
  (CallFunction|UpdateSegment)
  (Transformation|SetWorldLocation (Variables|Default|GetSMtarget) (Spline|GetLocationatTime (Variables|Default|GetSpline) 1.0 "World" false) false false))

(fn UpdateSegment
  (bind _spline (Variables|Default|GetSpline))
  (bind _instancercomponent (Variables|Default|GetInstancerComponent))
  (bind _instancercomponent_2 (Variables|Default|GetInstancerComponent))
  (bind _returnvalue (Spline|GetLocationatTime _spline 1.0 "World" false))
  (bind _returnvalue_2 (Transformation|GetWorldLocation _instancercomponent))
  (bind _returnvalue_3 (- _returnvalue _returnvalue_2))
  (bind _returnvalue_4 (Math|Vector|VectorLength _returnvalue_3))
  (bind _returnvalue_5 (Math|Vector|Normalize _returnvalue_3))
  (Variables|Instancing|SetTargDist _returnvalue_4)
  (if (> _returnvalue_4 0.0)
    (bind _output_get (Variables|Instancing|Setdirection _returnvalue_5))
    (if (Variables|Instancing|GetbOrientToTarget)
      (Variables|Instancing|Setrot (Math|Rotator|MakeRotfromX _returnvalue_5)))
    (bind _outtransformlist (Class|InstancerComponent|GenerateSerial _instancercomponent_2 (.ReturnValue (Math|Float|Division(WholeandRemainder) (Variables|Instancing|GetTargDist) (Variables|Instancing|GetStep))) (Math|Transform|MakeTransform (* _output_get (Variables|Instancing|GetStep)) "0, 0, 0" "1,1,1")))
    (bind _outtransformlist_2 (Class|InstancerComponent|ApplyModifierTransform _instancercomponent_2 _outtransformlist (Math|Transform|MakeTransform "0, 0, 0" (Variables|Instancing|Getrot) "1,1,1") false))
    (bind _outtransformlist_3 (Class|InstancerComponent|ApplyRandomizer _instancercomponent_2 _outtransformlist_2 (Utilities|Struct|MakeRandomizerOptions (Variables|Instancing|GetLocationVariance) (Variables|Instancing|GetRotationVariance) (Variables|Instancing|GetScaleVariance) false)))
    (Class|InstancerComponent|Realize _instancercomponent_2 _outtransformlist_3 (Variables|Instancing|GetInstancingMethod))
    (return)))